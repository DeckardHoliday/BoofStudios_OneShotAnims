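; BP_PlayerCharacter is the player Character, handling three-axis movement and camera look from input axes.
; MoveForward, MoveRight and MoveUp each add movement input along the capsule component's forward, right and up vectors, so movement follows the capsule's orientation.
; LookPitch and LookYaw feed their axis values straight into controller pitch and yaw.
; The construction script is empty.
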(event `InputAxis|MoveForward`
  (params (AxisValue :type "Float (single-precision)"))
  ;[1 1 1] X,Y,Z movement
  (`self.AddMovementInput` (`SceneComponent.GetForwardVector` (`self.CapsuleComponent`)) AxisValue))

(event `InputAxis|LookPitch`
  (params (AxisValue :type "Float (single-precision)"))
  ;[1 1 1] Camera Controls
  (`self.AddControllerPitchInput` AxisValue))

(event `InputAxis|LookYaw`
  (params (AxisValue :type "Float (single-precision)"))
  ;[1 1 1] Camera Controls
  (`self.AddControllerYawInput` AxisValue))

(event `InputAxis|MoveRight`
  (params (AxisValue :type "Float (single-precision)"))
  ;[1 1 1] X,Y,Z movement
  (`self.AddMovementInput` (`SceneComponent.GetRightVector` (`self.CapsuleComponent`)) AxisValue))

(event `InputAxis|MoveUp`
  (params (AxisValue :type "Float (single-precision)"))
  ;[1 1 1] X,Y,Z movement
  (`self.AddMovementInput` (`SceneComponent.GetUpVector` (`self.CapsuleComponent`)) AxisValue))

(fn `UserConstructionScript`)